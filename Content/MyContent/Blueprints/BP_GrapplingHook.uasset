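; Grappling hook projectile that flies out, then reels back to its owning player and destroys itself.
; An overlap with anything but itself or the player halts its movement, prints a catch message for BP_SpawnableCloud, then triggers the return.
; A two-second timeout disables overlaps and also triggers the return, which uses MoveComponentTo toward the player's location at that moment.
; The cable attachment to the player's mesh is unconnected.
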(event OnComponentBeginOverlap(Capsule)
  (params (OverlappedComponent :type Primitive%20Component%20Object%20Reference) (OtherActor :type Actor%20Object%20Reference) (OtherComp :type Primitive%20Component%20Object%20Reference) (OtherBodyIndex :type Integer) (bFromSweep :type Boolean) (SweepResult :type Hit%20Result%20Structure%20%28by%20ref%29))
  ;[1 1 1] Collision
  (if (and (!= self OtherActor) (!= OtherActor (Game|GetPlayerCharacter 0)))
    (Utilities|FlowControl|Delay 0.1)
    (CallFunction|StopProjectileMovement)
    (Utilities|FlowControl|Delay 0.3)
    (if (== (Utilities|GetClass OtherActor) "/Game/MyContent/Blueprints/BP_SpawnableCloud.BP_SpawnableCloud_C")
      (Development|PrintString "caught floating island"))
    (CallFunction|ReturntoPlayer)))

(event Custom|Return%20to%20Player
  ;[1 1 1] Return to Player
  (Variables|/Script/Engine.ProjectileMovementComponent|SetbRotationFollowsVelocity (Variables|Default|GetProjectileMovement) false)
  (Components|MoveComponentTo (Variables|Default|GetDefaultSceneRoot) (Transformation|GetActorLocation (Variables|Default|GetOwningPlayer)) (Transformation|GetActorRotation self) false false 0.5 false)
  (Actor|DestroyActor))

(event EventBeginPlay
  ;[1 1 1] InitSetup
  (Utilities|FlowControl|Delay 2.0)
  (Variables|/Script/Engine.PrimitiveComponent|SetbGenerateOverlapEvents (Variables|Default|GetCapsule) false)
  (CallFunction|ReturntoPlayer))

(fn ConstructionScript)

(fn StopProjectileMovement
  (bind _projectilemovement (Variables|Default|GetProjectileMovement))
  (Components|Movement|StopMovementImmediately _projectilemovement)
  (Variables|/Script/Engine.ProjectileMovementComponent|SetProjectileGravityScale _projectilemovement 0.0))