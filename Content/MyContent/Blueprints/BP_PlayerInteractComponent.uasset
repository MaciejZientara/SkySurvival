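; Player interaction component that detects what the camera is looking at and lets the player interact with it.
; Every tick, a debug-drawn visibility trace from the camera updates the looked-at actor.
; BP_LookAtComponent on old and new targets is notified to toggle outlines, and the HUD interact prompt is refreshed.
; IA_Interact sends InteractMessage to the target's first component implementing BPI_InteractInterface, passing the owning character.
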(event Custom|PlayerLookAtEvent
  (bind _returnvalue (Game|GetPlayerCameraManager 0))
  (bind _returnvalue_2 (Transformation|GetActorLocation _returnvalue))
  ;[1 1 1] PlayerLookAtEvent
  (bind _outhit (Collision|LineTraceByChannel _returnvalue_2 (+ _returnvalue_2 (* (Transformation|GetActorForwardVector _returnvalue) 1e+03)) "TraceTypeQuery1" false (Utilities|Array|MakeArray (Components|GetOwner)) "ForOneFrame"))
  (CallFunction|ProcessLookatObject (.HitActor (Collision|BreakHitResult _outhit))))

(event Input|EnhancedActionEvents|EnhancedInputActionIA_Interact
  (params (ActionValue :type Boolean) (ElapsedSeconds :type Float%20%28double-precision%29) (TriggeredSeconds :type Float%20%28double-precision%29) (InputAction :type Input%20Action%20Object%20Reference :default "/Game/MyContent/Inputs/Actions/IA_Interact.IA_Interact"))
  ;[1 1 1] Interact Event
  (:Started
    (bind _lookatobject (Variables|Default|GetLookAtObject)
      (:then
        (if (!= (Utilities|Array|Length (Class|Actor|GetComponentsbyInterface _lookatobject "/Game/MyContent/Interfaces/BPI_InteractInterface.BPI_InteractInterface_C")) 0)
          (Class|BPIInteractInterface|Interact(Message) (Utilities|Array|Get(acopy) (Class|Actor|GetComponentsbyInterface _lookatobject "/Game/MyContent/Interfaces/BPI_InteractInterface.BPI_InteractInterface_C")) (.AsBP%20Third%20Person%20Character (Utilities|Casting|CastToBP_ThirdPersonCharacter (Components|GetOwner))))))
      (:else))))

(event EventTick
  (params (DeltaSeconds :type Float%20%28single-precision%29))
  ;[1 1 1] Event Tick
  (CallFunction|PlayerLookatEvent))

(fn ProcessLookatObject
  (params (HitActor :type Actor%20Object%20Reference))
  (Utilities|FlowControl|Sequence
    (:then_0
      ;[1 1 1] Remove outline from previously looked at object
      (Utilities|IsValid (Variables|Default|GetLookAtObject) ; Is LookAtObject null?
        (:Is%20Valid
          (Utilities|IsValid (Actor|GetComponentbyClass (Variables|Default|GetLookAtObject) "/Game/MyContent/Inventory/BP_LookAtComponent.BP_LookAtComponent_C") ; Does LookAtObject have component?
            (:Is%20Valid
              (Class|BPILookatInterface|AfterLookat(Message) (Actor|GetComponentbyClass (Variables|Default|GetLookAtObject) "/Game/MyContent/Inventory/BP_LookAtComponent.BP_LookAtComponent_C")))))
        (:Is%20Not%20Valid
          _))
      (Default|RemovePresstoInteractWidget (Variables|/Game/MyContent/Blueprints/BP_HUDPlayerController.BP_HUDPlayerController_C|GetInventoryWidget (.AsBP%20HUDPlayer%20Controller (Utilities|Casting|CastToBP_HUDPlayerController (Game|GetPlayerController 0))))))
    (:then_1
      ;[1 1 1] Add outline to new looked at object
      (bind _output_get (Variables|Default|SetLookAtObject HitActor))
      (Utilities|IsValid _output_get ; Is LookAtObject null?
        (:Is%20Valid
          (Utilities|IsValid (Actor|GetComponentbyClass _output_get "/Game/MyContent/Inventory/BP_LookAtComponent.BP_LookAtComponent_C") ; Does LookAtObject have component?
            (:Is%20Valid
              (Class|BPILookatInterface|Lookat(Message) (Actor|GetComponentbyClass _output_get "/Game/MyContent/Inventory/BP_LookAtComponent.BP_LookAtComponent_C"))
              (Default|AddPresstoInteractWidget (Variables|/Game/MyContent/Blueprints/BP_HUDPlayerController.BP_HUDPlayerController_C|GetInventoryWidget (.AsBP%20HUDPlayer%20Controller (Utilities|Casting|CastToBP_HUDPlayerController (Game|GetPlayerController 0))))))))))))