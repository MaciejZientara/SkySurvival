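; Building system component for the third-person character that shows a placement preview while build mode is toggled on with IA_Build.
; Each tick in build mode, a camera-forward line trace moves a green, collision-free box mesh to the hit point.
; A DoOnce spawns the preview on the owning character at the first hit; exiting clears its mesh and reference without destroying the component, then resets the gate.
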(event Custom|Preview%20Loop
  (bind _returnvalue (Game|GetPlayerCameraManager 0))
  (bind _returnvalue_2 (Camera|GetCameraLocation _returnvalue))
  (bind (_outhit _returnvalue_3) (Collision|LineTraceByChannel _returnvalue_2 (+ _returnvalue_2 (* (Math|Vector|GetForwardVector (Camera|GetCameraRotation _returnvalue)) 1e+03)) "TraceTypeQuery1" false 0 "ForOneFrame"))
  (if _returnvalue_3
    (Utilities|FlowControl|Sequence
      (:then_0
        (Utilities|FlowControl|DoOnce false
          (:Completed
            (bind _returnvalue_4 (Game|AddComponentbyClass (Variables|Default|GetBP%20Player) "/Script/Engine.StaticMeshComponent" false (Variables|Default|GetBuilding%20Preview%20Transform)))
            (bind _output_get (Variables|Default|SetPreview%20Mesh _returnvalue_4))
            (Components|StaticMesh|SetStaticMesh _output_get "/ControlRig/Controls/ControlRig_Box_solid.ControlRig_Box_solid")
            (Rendering|Material|SetMaterial (Variables|Default|GetPreview%20Mesh) 0 "/Game/MyContent/Materials/M_PreviewGreen.M_PreviewGreen")
            (Collision|SetCollisionEnabled (Variables|Default|GetPreview%20Mesh) "NoCollision") ; Remove Collision
          )))
      (:then_1
        (bind _output_get_2 (Variables|Default|SetBuilding%20Preview%20Transform (Math|Transform|MakeTransform (.Location (Collision|BreakHitResult _outhit)) "0, 0, 0" "1.000000,1.000000,1.000000")))
        (Transformation|SetWorldTransform (Variables|Default|GetPreview%20Mesh) _output_get_2 false false)))))

(event Custom|ResetBuildMode
  (Utilities|FlowControl|DoOnce false) ; enters at Reset
)

(event Input|EnhancedActionEvents|EnhancedInputActionIA_Build
  (params (ActionValue :type Boolean) (ElapsedSeconds :type Float%20%28double-precision%29) (TriggeredSeconds :type Float%20%28double-precision%29) (InputAction :type Input%20Action%20Object%20Reference :default "/Game/MyContent/Inputs/Actions/IA_Build.IA_Build"))
  (:Started
    (bind _output_get (Variables|Default|SetIsBuildMode (not (Variables|Default|GetIsBuildMode))))
    (if (not _output_get)
      ;[1 1 1] Set Preview Mesh to NULL on exit build mode
      (bind _preview_mesh (Variables|Default|GetPreview%20Mesh) ; Is mesh not null?
        (:then
          (Components|StaticMesh|SetStaticMesh _preview_mesh 0)
          (Variables|Default|SetPreview%20Mesh 0)
          (CallFunction|ResetBuildMode))
        (:else)))))

(event EventBeginPlay
  (bind _asbp_third_person_character (Utilities|Casting|CastToBP_ThirdPersonCharacter (Components|GetOwner)))
  (Variables|Default|SetBP%20Player _asbp_third_person_character))

(event EventTick
  (params (DeltaSeconds :type Float%20%28single-precision%29))
  (if (Variables|Default|GetIsBuildMode)
    (CallFunction|PreviewLoop)))