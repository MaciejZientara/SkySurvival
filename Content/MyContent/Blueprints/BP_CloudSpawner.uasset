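; BP_CloudSpawner populates the level with BP_SpawnableCloud actors and keeps adding more during play.
; BeginPlay pre-fills the scene with clouds at randomized X positions, then loops forever on a randomized retriggerable delay, spawning one cloud at a fixed far X each time.
; SpawnCloud randomizes Y and Z distances, each scaled by a random MultiplyMap lookup, and optionally re-randomizes X after spawning for the initial fill.
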(event Custom|SpawnCloud
  (params (SetRandomX :type Boolean))
  (bind _returnvalue (Game|SpawnActorfromClass "/Game/MyContent/Blueprints/BP_SpawnableCloud.BP_SpawnableCloud_C" (Math|Conversions|ToTransform(Vector) (Math|Vector|MakeVector 1e+04 (* (.Value (Utilities|Map|Find (Variables|Default|GetMultiplyMap) (Math|Random|RandomIntegerinRange 0 1))) (Math|Random|RandomFloatinRange 1e+03 5e+03)) (* (Math|Random|RandomFloatinRange 1e+03 5e+03) (.Value (Utilities|Map|Find (Variables|Default|GetMultiplyMap) (Math|Random|RandomIntegerinRange 0 1)))))) "Undefined" "MultiplyWithRoot" 0 0))
  (if SetRandomX
    (Transformation|SetActorLocation _returnvalue (Math|Vector|MakeVector (Math|Random|RandomFloatinRange -8e+03 8e+03) (.y (Transformation|GetActorLocation _returnvalue)) (.z (Transformation|GetActorLocation _returnvalue))) false false)))

(event EventBeginPlay
  (for _index (range 0 100)
    (CallFunction|SpawnCloud true))
  (Utilities|FlowControl|RetriggerableDelay (Math|Random|RandomFloatinRange 1.0 5.0) :!label _label)
  (CallFunction|SpawnCloud false)
  (goto _label))

(event Collision|EventActorBeginOverlap
  (params (OtherActor :type Actor%20Object%20Reference)))

(event EventTick
  (params (DeltaSeconds :type Float%20%28single-precision%29)))

(fn ConstructionScript)