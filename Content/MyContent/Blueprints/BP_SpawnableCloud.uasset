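; BP_SpawnableCloud is a cloud actor that drifts along negative X at a random speed chosen on BeginPlay.
; A self-calling Movement event offsets its location every 0.02 seconds.
; It destroys itself only when the next X exactly equals -10000, a float comparison the random speed can easily skip.
; BeginPlay also adds two static mesh components, with a separate pair on a 1-in-100 roll.
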(event Custom|Movement
  (bind _returnvalue (Transformation|GetActorLocation))
  (bind _speed (Variables|Default|GetSpeed))
  (bind _returnvalue_2 (+ _returnvalue (Math|Vector|MakeVector _speed 0.0 0.0)))
  (Transformation|SetActorLocation _returnvalue_2 false false)
  (if (== (.X (Math|Vector|BreakVector _returnvalue_2)) -1e+04)
    (Actor|DestroyActor)
    (else
      (Utilities|FlowControl|Delay 0.02)
      (CallFunction|Movement))))

(event EventBeginPlay
  (Variables|Default|SetSpeed (Math|Random|RandomFloatinRange -1.0 -5.0))
  (CallFunction|Movement)
  (if (== (Math|Random|RandomInteger 100) 0)
    (AddComponent|AddStaticMeshComponent false)
    (AddComponent|AddStaticMeshComponent false)
    (else
      (AddComponent|AddStaticMeshComponent false)
      (AddComponent|AddStaticMeshComponent false))))

(fn ConstructionScript)