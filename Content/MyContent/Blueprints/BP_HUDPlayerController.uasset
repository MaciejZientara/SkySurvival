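; Player controller that creates the stamina and inventory HUD for the third-person character and handles hotbar selection and item pickup.
; Scroll input cycles a wrapping nine-slot highlight on the hotbar grid.
; Pickup makes two add attempts, both on the main inventory despite a commented hotbar fallback, then shows a full-inventory popup for leftovers.
; Server-named events write inventory content and item quantity, destroying emptied item actors the client does not own.
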(event Custom|ServerUpdateContent
  (params (Content :type Array%20of%20Inventory%20Slot%20Struct%20Structures) (InventoryComponent :type BP%20Inventory%20Content%20Object%20Reference))
  ;[1 1 1] Server update client item/inventory
  (Variables|/Game/MyContent/Inventory/BP_InventoryContent.BP_InventoryContent_C|SetContent InventoryComponent Content))

(event Custom|TryAddItemInventory
  (params (ItemComponent :type BP%20Item%20Component%20Object%20Reference))
  (bind _quantity (Variables|/Game/MyContent/Inventory/BP_ItemComponent.BP_ItemComponent_C|GetQuantity ItemComponent))
  (bind _itemhandle (Variables|/Game/MyContent/Inventory/BP_ItemComponent.BP_ItemComponent_C|GetItemHandle ItemComponent))
  ;[1 1 1] Try to add to inventory, else try to add to hotbar, else full inventory popup
  (Utilities|FlowControl|Sequence
    (:then_0
      (if (> _quantity 0)
        (bind _remainingquantity (Default|AddItem (Variables|/Game/MyContent/Blueprints/BP_ThirdPersonCharacter.BP_ThirdPersonCharacter_C|GetInventorySystem%28inventory%29 (Variables|Default|GetPlayerRef)) _itemhandle _quantity))))
    (:then_1
      (if (> _remainingquantity 0)
        (bind _remainingquantity_2 (Default|AddItem (Variables|/Game/MyContent/Blueprints/BP_ThirdPersonCharacter.BP_ThirdPersonCharacter_C|GetInventorySystem%28inventory%29 (Variables|Default|GetPlayerRef)) _itemhandle _remainingquantity))))
    (:then_2
      (Utilities|FlowControl|Sequence
        (:then_0
          (if (> _remainingquantity_2 0)
            (Default|FullInventoryPopup (Variables|Default|GetInventoryWidget))))
        (:then_1
          (CallFunction|CallServerUpdateItemActor ItemComponent _remainingquantity_2)
          ;;[1 1 1] Remove PressToInteract widget when item removed
          (if (== 0 _remainingquantity_2)
            (Default|RemovePresstoInteractWidget (Variables|Default|GetInventoryWidget))))))))

(event Custom|CallServerUpdateItemActor
  (params (ItemComponent :type BP%20Item%20Component%20Object%20Reference) (Quantity :type Integer))
  ;[1 1 1] Server update client item/inventory
  ;;[1 1 1] Item Actor is not owning client, update/destroy of item needs to be done by player character or its components
  (CallFunction|ServerUpdateItemActor ItemComponent Quantity))

(event Custom|ServerUpdateItemActor
  (params (ItemComponent :type BP%20Item%20Component%20Object%20Reference) (Quantity :type Integer))
  ;[1 1 1] Server update client item/inventory
  ;;[1 1 1] Item Actor is not owning client, update/destroy of item needs to be done by player character or its components
  (bind _output_get (Variables|/Game/MyContent/Inventory/BP_ItemComponent.BP_ItemComponent_C|SetQuantity ItemComponent Quantity))
  (if (== _output_get 0)
    (Actor|DestroyActor (Components|GetOwner ItemComponent))))

(event Input|EnhancedActionEvents|EnhancedInputActionIA_RMB
  (params (ActionValue :type Boolean) (ElapsedSeconds :type Float%20%28double-precision%29) (TriggeredSeconds :type Float%20%28double-precision%29) (InputAction :type Input%20Action%20Object%20Reference :default "/Game/MyContent/Inputs/Actions/IA_RMB.IA_RMB"))
  ;[1 1 1] Use Item Hotbar Selected Slot
)

(event Input|EnhancedActionEvents|EnhancedInputActionIA_LMB
  (params (ActionValue :type Boolean) (ElapsedSeconds :type Float%20%28double-precision%29) (TriggeredSeconds :type Float%20%28double-precision%29) (InputAction :type Input%20Action%20Object%20Reference :default "/Game/MyContent/Inputs/Actions/IA_LMB.IA_LMB"))
  ;[1 1 1] Use Item Hotbar Selected Slot
)

(event Input|EnhancedActionEvents|EnhancedInputActionIA_ScrollHotbar
  (params (ActionValue :type Float%20%28double-precision%29) (ElapsedSeconds :type Float%20%28double-precision%29) (TriggeredSeconds :type Float%20%28double-precision%29) (InputAction :type Input%20Action%20Object%20Reference :default "/Game/MyContent/Inputs/Actions/IA_ScrollHotbar.IA_ScrollHotbar"))
  ;[1 1 1] Scroll Hotbar
  (:Started
    (Math|Float|CompareFloat ActionValue 0.0
      (:>
        (CallFunction|SetHotbarSlotColor (Math|Integer|%(Integer) (+ (Variables|Default|GetHotbarSlotIndex) 8) 9)))
      (:<
        (CallFunction|SetHotbarSlotColor (Math|Integer|%(Integer) (+ (Variables|Default|GetHotbarSlotIndex) 1) 9))))))

(event EventBeginPlay
  (bind _asbp_third_person_character (Utilities|Casting|CastToBP_ThirdPersonCharacter (Pawn|GetControlledPawn self)))
  (bind _output_get (Variables|Default|SetPlayerRef _asbp_third_person_character))
  ;[1 1 1] Add sprint HUD
  (bind _returnvalue (UserInterface|CreateWidget "/Game/MyContent/Stamina/WBP_StaminaHUD.WBP_StaminaHUD_C" 0 _output_get))
  (bind _output_get_2 (Variables|Default|SetSprintHUD _returnvalue))
  (UserInterface|Viewport|AddtoViewport _output_get_2 0)
  (CallFunction|InventoryInit))

(fn ConstructionScript)

(fn InventoryInit
  (bind _returnvalue (UserInterface|CreateWidget "/Game/MyContent/Inventory/WBP_PlayerInventoryWidget.WBP_PlayerInventoryWidget_C"))
  (bind _output_get (Variables|Default|SetInventoryWidget _returnvalue))
  (UserInterface|Viewport|AddtoViewport _output_get 0)
  (Utilities|FlowControl|Sequence
    (:then_0
      (Default|UpdateGrid (Variables|/Game/MyContent/Blueprints/BP_ThirdPersonCharacter.BP_ThirdPersonCharacter_C|GetInventorySystem%28inventory%29 (Variables|Default|GetPlayerRef))))
    (:then_1
      (Default|UpdateGrid (Variables|/Game/MyContent/Blueprints/BP_ThirdPersonCharacter.BP_ThirdPersonCharacter_C|GetInventorySystem%28Hotbar%29 (Variables|Default|GetPlayerRef))))
    (:then_2
      ;[1 1 1] Set first hotbar slot to set
      (CallFunction|SetHotbarSlotColor))))

(fn SetHotbarSlotColor
  (params (SlotIndex :type Integer))
  (LocalVariables|SetGrid (Variables|/Game/MyContent/Inventory/WBP_InventoryGridClass.WBP_InventoryGridClass_C|GetGrid (Variables|/Game/MyContent/Inventory/WBP_PlayerInventoryWidget.WBP_PlayerInventoryWidget_C|GetHotbar (Variables|Default|GetInventoryWidget))))
  (Utilities|FlowControl|Sequence
    (:then_0
      (bind _aswbp_item_slot_class (Utilities|Casting|CastToWBP_ItemSlotClass (Class|PanelWidget|GetChildat (LocalVariables|GetGrid) (Variables|Default|GetHotbarSlotIndex))))
      (bind _output_get (Variables|/Game/MyContent/Inventory/WBP_ItemSlotClass.WBP_ItemSlotClass_C|SetIsColored _aswbp_item_slot_class false))
      (Default|SetColor _aswbp_item_slot_class _output_get))
    (:then_1
      (bind _output_get_2 (Variables|Default|SetHotbarSlotIndex SlotIndex))
      (bind _aswbp_item_slot_class_2 (Utilities|Casting|CastToWBP_ItemSlotClass (Class|PanelWidget|GetChildat (LocalVariables|GetGrid) _output_get_2)))
      (bind _output_get_3 (Variables|/Game/MyContent/Inventory/WBP_ItemSlotClass.WBP_ItemSlotClass_C|SetIsColored _aswbp_item_slot_class_2 true))
      (Default|SetColor _aswbp_item_slot_class_2 _output_get_3))))