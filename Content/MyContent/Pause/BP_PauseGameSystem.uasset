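; BP_PauseGameSystem toggles the game's pause state from the PauseGame input action or a TogglePause event.
; When pausing, it freezes the game, creates a WBP_PauseMenu widget, and switches to game-and-UI input focused on the menu with the mouse cursor shown.
; When resuming, it removes the menu, restores game-only input and hides the cursor.
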(event Custom|TogglePause
  (bind _returnvalue (Game|GetPlayerController 0))
  ;[1 1 1] PauseGame
  (bind _output_get (Variables|Default|SetIsGamePaused (not (Variables|Default|GetIsGamePaused))))
  (Game|SetGamePaused _output_get)
  (if _output_get
    (bind _returnvalue_2 (UserInterface|CreateWidget "/Game/MyContent/Pause/WBP_PauseMenu.WBP_PauseMenu_C" _returnvalue))
    (bind _output_get_2 (Variables|Default|SetPauseMenuWidget _returnvalue_2))
    (UserInterface|Viewport|AddtoViewport _output_get_2 0)
    (Input|SetInputModeGameandUI _returnvalue (Variables|Default|GetPauseMenuWidget) "DoNotLock" true false)
    (Variables|/Script/Engine.PlayerController|SetbShowMouseCursor (Game|GetPlayerController 0) true)
    (else
      (Widget|RemovefromParent (Variables|Default|GetPauseMenuWidget))
      (Input|SetInputModeGameOnly _returnvalue false)
      (Variables|/Script/Engine.PlayerController|SetbShowMouseCursor (Game|GetPlayerController 0) false))))

(event Input|EnhancedActionEvents|EnhancedInputActionPauseGame
  (params (ActionValue :type Boolean) (ElapsedSeconds :type Float%20%28double-precision%29) (TriggeredSeconds :type Float%20%28double-precision%29) (InputAction :type Input%20Action%20Object%20Reference :default "/Game/MyContent/Inputs/Actions/PauseGame.PauseGame"))
  (bind _returnvalue (Game|GetPlayerController 0))
  ;[1 1 1] PauseGame
  (:Started
    (bind _output_get (Variables|Default|SetIsGamePaused (not (Variables|Default|GetIsGamePaused))))
    (Game|SetGamePaused _output_get)
    (if _output_get
      (bind _returnvalue_2 (UserInterface|CreateWidget "/Game/MyContent/Pause/WBP_PauseMenu.WBP_PauseMenu_C" _returnvalue))
      (bind _output_get_2 (Variables|Default|SetPauseMenuWidget _returnvalue_2))
      (UserInterface|Viewport|AddtoViewport _output_get_2 0)
      (Input|SetInputModeGameandUI _returnvalue (Variables|Default|GetPauseMenuWidget) "DoNotLock" true false)
      (Variables|/Script/Engine.PlayerController|SetbShowMouseCursor (Game|GetPlayerController 0) true)
      (else
        (Widget|RemovefromParent (Variables|Default|GetPauseMenuWidget))
        (Input|SetInputModeGameOnly _returnvalue false)
        (Variables|/Script/Engine.PlayerController|SetbShowMouseCursor (Game|GetPlayerController 0) false)))))