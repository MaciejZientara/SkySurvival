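; Stamina component for BP_ThirdPersonCharacter that doubles max walk speed while IA_Sprint is held and drops it back when stamina runs out.
; Tick detects movement and triggers a drain while sprinting, throttled by a Delay.
; A self-calling delayed event started at BeginPlay regenerates stamina, faster standing than moving, and pauses while sprint is held in motion, even at zero stamina.
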(event Custom|Stop%20Running
  ;[1 1 1] Stop Running
  (Variables|/Script/Engine.CharacterMovementComponent|SetMaxWalkSpeed (Variables|Default|GetCharacter%20Movement) (Variables|Default|GetPlayer%20Max%20Walk%20Speed)))

(event Custom|Start%20Running
  ;[1 1 1] Start Running
  (Variables|/Script/Engine.CharacterMovementComponent|SetMaxWalkSpeed (Variables|Default|GetCharacter%20Movement) (* (Variables|Default|GetPlayer%20Max%20Walk%20Speed) 2.0)))

(event Custom|Stamina%20Up
  (bind _maxstamina (Variables|Default|GetMaxStamina))
  ;[1 1 1] Stamina UP (0 when running, slower rate up when moving, faster rate up while standing)
  (Utilities|FlowControl|Delay 0.2)
  (if (and (Variables|Default|GetIs%20Sprinting?) (Variables|Default|GetIsMoving?))
    _
    (elif (Variables|Default|GetIsMoving?)
      (Variables|Default|SetStamina (Math|Integer|Clamp(Integer) (+ 1 (Variables|Default|GetStamina)) 0 _maxstamina))
      (else
        (Variables|Default|SetStamina (Math|Integer|Clamp(Integer) (+ 5 (Variables|Default|GetStamina)) 0 _maxstamina)))))
  (CallFunction|StaminaUp))

(event Custom|Stamina%20Down
  ;[1 1 1] Stamina Down
  (Utilities|FlowControl|Delay 0.2)
  (bind _output_get (Variables|Default|SetStamina (Math|Integer|Clamp(Integer) (- (Variables|Default|GetStamina) 2) 0 (Variables|Default|GetMaxStamina))))
  (if (== _output_get 0)
    (CallFunction|StopRunning)))

(event Input|EnhancedActionEvents|EnhancedInputActionIA_Sprint
  (params (ActionValue :type Boolean) (ElapsedSeconds :type Float%20%28double-precision%29) (TriggeredSeconds :type Float%20%28double-precision%29) (InputAction :type Input%20Action%20Object%20Reference :default "/Game/MyContent/Inputs/Actions/IA_Sprint.IA_Sprint"))
  ;[1 1 1] Sprint with Stamina
  (:Started
    (CallFunction|StartRunning)
    (Variables|Default|SetIs%20Sprinting? true))
  (:Completed
    (CallFunction|StopRunning)
    (Variables|Default|SetIs%20Sprinting? false)))

(event EventBeginPlay
  ;[1 1 1] Init
  (CallFunction|StaminaUp)
  ;;[1 1 1] Set Default Max Walk Speed to variable
  (bind _output_get (Variables|Default|SetCharacter%20Movement (Variables|/Script/Engine.Character|GetCharacterMovement (.AsBP%20Third%20Person%20Character (Utilities|Casting|CastToBP_ThirdPersonCharacter (Components|GetOwner))))))
  (Variables|Default|SetPlayer%20Max%20Walk%20Speed (Variables|/Script/Engine.CharacterMovementComponent|GetMaxWalkSpeed _output_get)))

(event EventTick
  (params (DeltaSeconds :type Float%20%28single-precision%29))
  ;[1 1 1] Event Tick
  ;;[1 1 1] Check if character moving
  (Variables|Default|SetIsMoving? (> (Math|Vector|VectorLength (Variables|/Script/Engine.MovementComponent|GetVelocity (Variables|Default|GetCharacter%20Movement))) 0.0))
  (if (and (Variables|Default|GetIs%20Sprinting?) (Variables|Default|GetIsMoving?))
    (CallFunction|StaminaDown)))