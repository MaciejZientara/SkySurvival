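; BP_ItemComponent makes its owning actor a pickup item, carrying an item handle and quantity for the inventory system.
; On BeginPlay it turns on replication for the owner.
; Interact passes the component to the player's BP_HUDPlayerController through TryAddItemInventory.
; TryToAddItem adds any positive quantity to the given inventory system and stores the remainder locally until the server's global update.
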(event EventBeginPlay
  ;[1 1 1] Set item replication
  (Networking|SetReplicates (Components|GetOwner) true))

(event EventInteract
  (params (PlayerReferance :type BP%20Third%20Person%20Character%20Object%20Reference))
  ;[1 1 1] TryAddItem in Player Controller
  (bind _asbp_hudplayer_controller (Utilities|Casting|CastToBP_HUDPlayerController (Pawn|GetController PlayerReferance)))
  (Default|TryAddItemInventory _asbp_hudplayer_controller self))

(fn TrytoAddItem
  (params (InventorySystem :type BP%20Inventory%20Content%20Object%20Reference))
  (if (> (Variables|Default|GetQuantity) 0)
    (bind _remainingquantity (Default|AddItem InventorySystem (Variables|Default|GetItemHandle) (Variables|Default|GetQuantity)))
    (Variables|Default|SetQuantity _remainingquantity) ; update for local check purpose, will be updated globaly by server later
  ))