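; BP_ChestComponent is a chest component that opens the player's inventory UI with the chest panel when interacted with.
; Interact reaches the inventory widget through the player's HUD controller, toggles its visibility and shows the Chest grid.
; It links that grid to the owner's BP_InventoryContent, rebuilding slots only when that differs from the one already bound.
; The grid's content refreshes on every interaction.
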(event EventInteract
  (params (PlayerReferance :type BP%20Third%20Person%20Character%20Object%20Reference))
  (bind _returnvalue (Components|GetOwner))
  (bind _returnvalue_2 (Pawn|GetController PlayerReferance))
  (bind _returnvalue_3 (Actor|GetComponentbyClass _returnvalue "/Game/MyContent/Inventory/BP_InventoryContent.BP_InventoryContent_C"))
  (bind _asbp_hudplayer_controller (Utilities|Casting|CastToBP_HUDPlayerController _returnvalue_2))
  (bind _inventorywidget (Variables|/Game/MyContent/Blueprints/BP_HUDPlayerController.BP_HUDPlayerController_C|GetInventoryWidget _asbp_hudplayer_controller))
  (bind _chest (Variables|/Game/MyContent/Inventory/WBP_PlayerInventoryWidget.WBP_PlayerInventoryWidget_C|GetChest _inventorywidget))
  (Default|ChangeVisibility _inventorywidget)
  (Widget|SetVisibility _chest "Visible")
  ;[1 1 1] Aktualizuj slots tylko kiedy inny inventory component niż do tej pory (nie aktualizuj jesli otwierasz ta sama skrzynie)
  (if (!= (Variables|/Game/MyContent/Inventory/WBP_InventoryGridClass.WBP_InventoryGridClass_C|GetInventoryComponent _chest) _returnvalue_3)
    (bind _output_get (Variables|/Game/MyContent/Inventory/WBP_InventoryGridClass.WBP_InventoryGridClass_C|SetInventoryComponent _chest _returnvalue_3))
    (Variables|/Game/MyContent/Inventory/BP_InventoryContent.BP_InventoryContent_C|SetGridWidget _output_get _chest)
    (Default|UpdateSlots _chest))
  (Default|UpdateContent _chest))