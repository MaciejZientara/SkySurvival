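; Inventory component that holds a fixed-size array of item slots, sized from GridSize on BeginPlay.
; AddItem looks up the DataTable row, tops up matching stacks before filling empty slots up to max stack size, and returns any remainder.
; After each slot change, UpdateGrid refreshes the grid widget and pushes the locally edited content to the server through player controller 0.
; RemoveItem is an empty stub.
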(event Custom|UpdateGrid
  ;[1 1 1] Update Inventory client (widget) and server (content)
  (Default|UpdateContent (Variables|Default|GetGridWidget)) ; Update inventory widget
  (Default|ServerUpdateContent (.AsBP%20HUDPlayer%20Controller (Utilities|Casting|CastToBP_HUDPlayerController (Game|GetPlayerController 0))) (Variables|Default|GetContent) self) ; Update inventory content on server
)

(event EventBeginPlay
  ;[1 1 1] Set default size of content table
  (Utilities|Array|Resize (Variables|Default|GetContent) (Variables|Default|GetGridSize)))

(fn AddItem
  (params (ItemHandle :type Data%20Table%20Row%20Handle%20Structure) (Quantity :type Integer))
  (bind (_datatable _rowname) (Utilities|Struct|BreakDataTableRowHandle ItemHandle))
  (bind _returnvalue (Utilities|GetDataTableRow _datatable _rowname)
    (:then
      (bind _output_get (LocalVariables|SetRemaining%20Quantity Quantity))
      (while (> _output_get 0)
        (bind (_slotindex _availablequantity _foundslot _emptyslot) (CallFunction|FindSlot ItemHandle))
        (if _foundslot
          (if _emptyslot
            (CallFunction|NewIteminSlot _slotindex _returnvalue (Math|Integer|Min(Integer) _availablequantity (LocalVariables|GetRemaining%20Quantity)))
            (else
              (CallFunction|AddItemtoSlot _slotindex (Math|Integer|Min(Integer) _availablequantity (LocalVariables|GetRemaining%20Quantity)))))
          (LocalVariables|SetRemaining%20Quantity (- (LocalVariables|GetRemaining%20Quantity) (Math|Integer|Min(Integer) _availablequantity (LocalVariables|GetRemaining%20Quantity))))
          (CallFunction|UpdateGrid)
          (else
            (Development|PrintString "couldn't take item")
            (return false (LocalVariables|GetRemaining%20Quantity)) ; Couldn't take item
          )))
      (Development|PrintString "fully stored item")
      (return true 0) ; fully stored items
    )
    (:RowNotFound
      (Development|PrintString "row not found in table")
      (return false Quantity) ; row not found in table
    )))

(fn RemoveItem)

(fn FindSlot
  (params (ItemHandle :type Data%20Table%20Row%20Handle%20Structure))
  (bind (_datatable _rowname) (Utilities|Struct|BreakDataTableRowHandle ItemHandle))
  (bind _returnvalue (Utilities|GetDataTableRow _datatable _rowname)
    (:then
      ;[1 1 1] Find Slot with item and count != Max stack size
      (for (_array_element _array_index) (Variables|Default|GetContent)
        (if (and (> (- (.MaxStackSize (Utilities|Struct|BreakItemStructure (.Item (Utilities|Struct|BreakInventorySlotStruct _array_element)))) (.Count (Utilities|Struct|BreakInventorySlotStruct _array_element))) 0) (Utilities|Enum|Equal(Enum) (.Name (Utilities|Struct|BreakItemStructure (.Item (Utilities|Struct|BreakInventorySlotStruct _array_element)))) (.Name (Utilities|Struct|BreakItemStructure _returnvalue))))
          (return _array_index (- (.MaxStackSize (Utilities|Struct|BreakItemStructure (.Item (Utilities|Struct|BreakInventorySlotStruct _array_element)))) (.Count (Utilities|Struct|BreakInventorySlotStruct _array_element))) true false)))
      ;[1 1 1] Find Empty Slot
      (for (_array_element_2 _array_index_2) (Variables|Default|GetContent)
        (if (== (.Count (Utilities|Struct|BreakInventorySlotStruct _array_element_2)) 0)
          (return _array_index_2 (.MaxStackSize (Utilities|Struct|BreakItemStructure _returnvalue)) true true)))
      (return 0 0 false false) ; Not Found Empty Slot
    )))

(fn AddItemtoSlot
  (params (SlotIndex :type Integer) (Quantity :type Integer))
  (bind _content (Variables|Default|GetContent))
  (bind _output (Utilities|Array|Get(acopy) _content SlotIndex))
  (bind (_count _item) (Utilities|Struct|BreakInventorySlotStruct _output))
  (Utilities|Array|SetArrayElem (Variables|Default|GetContent) SlotIndex (Utilities|Struct|MakeInventorySlotStruct (+ Quantity _count) _item)))

(fn NewIteminSlot
  (params (SlotIndex :type Integer) (Item :type Item%20Structure%20Structure) (Quantity :type Integer))
  (Utilities|Array|SetArrayElem (Variables|Default|GetContent) SlotIndex (Utilities|Struct|MakeInventorySlotStruct Quantity Item)))

(fn DEBUGprintContent
  (for (_array_element _array_index) (Variables|Default|GetContent)
    (Development|PrintText (Utilities|Text|FormatText "{idx}: ({name},{count})" _array_index (.Name (Utilities|Struct|BreakItemStructure (.Item (Utilities|Struct|BreakInventorySlotStruct _array_element)))) (.Count (Utilities|Struct|BreakInventorySlotStruct _array_element))))))