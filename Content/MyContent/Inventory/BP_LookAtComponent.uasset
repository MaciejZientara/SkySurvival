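; BP_LookAtComponent is a component that switches an outline highlight on and off for its owning actor, driven by look-at events.
; Lookat sets M_OutlineOverlay as the overlay material on every mesh component among the root component's descendants, and AfterLookat clears it.
; Both events gather those children recursively at call time, so the root component itself is not affected.
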(event EventAfterLookat
  ;[1 1 1] Remove Overlay Material
  (for _array_element (Components|GetChildrenComponents (Variables|/Script/Engine.Actor|GetRootComponent (Components|GetOwner)) true)
    (bind _asmesh_component (Utilities|Casting|CastToMeshComponent _array_element))
    (Rendering|Material|SetOverlayMaterial _asmesh_component 0 :!class /Script/Engine.MeshComponent)))

(event EventLookat
  ;[1 1 1] Add Overlay Material
  (for _array_element (Components|GetChildrenComponents (Variables|/Script/Engine.Actor|GetRootComponent (Components|GetOwner)) true)
    (bind _asmesh_component (Utilities|Casting|CastToMeshComponent _array_element))
    (Rendering|Material|SetOverlayMaterial _asmesh_component "/Game/MyContent/Materials/M_OutlineOverlay.M_OutlineOverlay" :!class /Script/Engine.MeshComponent)))