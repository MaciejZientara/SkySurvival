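; BP_DeathRebirthComponent is a component for BP_ThirdPersonCharacter that handles death and respawn when the player falls out of the world.
; Tick checks the owner's height and calls Death below a Z threshold, guarded by an IsDead flag.
; Death shows a BPI_Death widget, then after a short delay Rebirth removes it, forces garbage collection and teleports the same character to a PlayerStart rather than spawning a new one.
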(event Custom|Death
  ;[1 1 1] TODO: change to GUI "U DIED" screen
  (if (not (Variables|Default|GetIsDead))
    (Variables|Default|SetIsDead true)
    (bind _returnvalue (UserInterface|CreateWidget "/Game/MyContent/Death/BPI_Death.BPI_Death_C"))
    (bind _output_get (Variables|Default|SetDeathWidget _returnvalue))
    (UserInterface|Viewport|AddtoViewport _output_get 0)
    (Utilities|FlowControl|Delay 1.0)
    (CallFunction|Rebirth)))

(event Custom|Rebirth
  ;[1 1 1] TODO: Change to destroy player + spawn new player
  (Widget|RemovefromParent (Variables|Default|GetDeathWidget))
  (Utilities|Platform|CollectGarbage)
  (bind _returnvalue (Actor|GetActorOfClass "/Script/Engine.PlayerStart"))
  (Transformation|SetActorLocation (Variables|Default|GetPlayerRef) (Transformation|GetActorLocation _returnvalue) false true)
  (Variables|Default|SetIsDead false))

(event EventBeginPlay
  (bind _asbp_third_person_character (Utilities|Casting|CastToBP_ThirdPersonCharacter (Components|GetOwner)))
  (Variables|Default|SetPlayerRef _asbp_third_person_character))

(event EventTick
  (params (DeltaSeconds :type Float%20%28single-precision%29))
  (if (< (.z (Transformation|GetActorLocation (Variables|Default|GetPlayerRef))) -5e+03)
    (CallFunction|Death)))